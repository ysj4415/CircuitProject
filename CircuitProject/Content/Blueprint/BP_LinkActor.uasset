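; BP_LinkActor draws a cable between two child actors, StartPoint and EndPoint.
; On BeginPlay it attaches the Cable component's end to the EndPoint child actor.
; Every Tick, SetCableLocation moves the cable's origin to the StartPoint child actor's world location, so the cable follows that end.
; An alternative manual EndLocation calculation remains in SetCableLocation but never runs.
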(event EventBeginPlay
  (Class|CableComponent|SetAttachEndto (Variables|Default|GetCable) (Variables|/Script/Engine.ChildActorComponent|GetChildActor (Variables|Default|GetEndPoint)) "None" "None"))

(event Collision|EventActorBeginOverlap
  (params (OtherActor :type Actor%20Object%20Reference)))

(event EventTick
  (params (DeltaSeconds :type Float%20%28single-precision%29))
  (CallFunction|SetCableLocation))

(fn ConstructionScript)

(fn SetCableLocation
  (Transformation|SetWorldLocation (Variables|Default|GetCable) (Transformation|GetActorLocation (Variables|/Script/Engine.ChildActorComponent|GetChildActor (Variables|Default|GetStartPoint))) false false))