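; BP_Switch is a two-state switch actor with a rotating handle and a child actor on each side.
; The construction script offsets both child actors along Y by one cell width (FieldLength / CellCount), stores them as LeftPoint and RightPoint, and poses the handle from SwitchValue.
; TurnOn, TurnOff and ToggleSwitch flip the value and tilt the handle.
; DetachCHildActor forwards a DetachMessage to both side actors.
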(event EventBeginPlay
  (|CallParentFunction) ; 지금 이 노드는 비활성 상태입니다. \n핀을 끌어서 다른 노드를 연결하면 활성화됩니다.
)

(event Collision|EventActorBeginOverlap
  (params (OtherActor :type Actor%20Object%20Reference))
  (|CallParentFunction OtherActor) ; 지금 이 노드는 비활성 상태입니다. \n핀을 끌어서 다른 노드를 연결하면 활성화됩니다.
)

(event EventTick
  (params (DeltaSeconds :type Float%20%28single-precision%29))
  (|CallParentFunction DeltaSeconds) ; 지금 이 노드는 비활성 상태입니다. \n핀을 끌어서 다른 노드를 연결하면 활성화됩니다.
)

(event EventDetachCHildActor
  (Class|Attach|Detach(Message) (Variables|/Script/Engine.ChildActorComponent|GetChildActor (Variables|Default|GetRightActor)))
  (Class|Attach|Detach(Message) (Variables|/Script/Engine.ChildActorComponent|GetChildActor (Variables|Default|GetLeftActor))))

(fn ConstructionScript
  (bind _fieldlength (Variables|Default|GetFieldLength))
  (bind _cellcount (Variables|Default|GetcellCount))
  (bind _sm_switchhandle (Variables|Default|GetSM_SwitchHandle))
  (bind _returnvalue (/ _fieldlength _cellcount))
  (|CallParentFunction)
  (Transformation|SetRelativeLocation (Variables|Default|GetLeftActor) (Math|Vector|MakeVector 0.0 _returnvalue 0.0) false false)
  (Transformation|SetRelativeLocation (Variables|Default|GetRightActor) (Math|Vector|MakeVector 0.0 (* _returnvalue -1.0) 0.0) false false)
  (Variables|Default|SetLeftPoint (Variables|/Script/Engine.ChildActorComponent|GetChildActor (Variables|Default|GetLeftActor)))
  (Variables|Default|SetRightPoint (Variables|/Script/Engine.ChildActorComponent|GetChildActor (Variables|Default|GetRightActor)))
  (if (Variables|Default|GetSwitchValue)
    (Transformation|SetRelativeRotation _sm_switchhandle "0.000000,0.000000,-40.000000" false false)
    (else
      (Transformation|SetRelativeRotation _sm_switchhandle "0.000000,0.000000,40.000000" false false))))

(fn Turnon
  (Variables|Default|SetSwitchValue true)
  (Transformation|SetRelativeRotation (Variables|Default|GetSM_SwitchHandle) "0.000000,0.000000,-40.000000" false false))

(fn TurnOff
  (Variables|Default|SetSwitchValue false)
  (Transformation|SetRelativeRotation (Variables|Default|GetSM_SwitchHandle) "0.000000,0.000000,40.000000" false false))

(fn ToggleSwitch
  (if (Variables|Default|GetSwitchValue)
    (CallFunction|TurnOff)
    (else
      (CallFunction|Turnon))))