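; BP_Door is a sliding door that the player opens and closes with the interaction input while inside its Box trigger.
; Overlapping the Box shows a door prompt on a viewport widget and enables player input; leaving reverses both.
; A FlipFlop alternates a timeline that slides the mesh sideways forward and in reverse.
; Tick keeps the prompt hidden while the door is open.
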(event OnComponentBeginOverlap(Box)
  (params (OverlappedComponent :type Primitive%20Component%20Object%20Reference) (OtherActor :type Actor%20Object%20Reference) (OtherComp :type Primitive%20Component%20Object%20Reference) (OtherBodyIndex :type Integer) (bFromSweep :type Boolean) (SweepResult :type Hit%20Result%20Structure%20%28by%20ref%29))
  (Widget|SetVisibility (Variables|/Game/Widget/UserWidget.UserWidget_C|GetDoor (Variables|Default|GetWidget)) "Visible")
  (Input|EnableInput (Game|GetPlayerController 0)))

(event OnComponentEndOverlap(Box)
  (params (OverlappedComponent :type Primitive%20Component%20Object%20Reference) (OtherActor :type Actor%20Object%20Reference) (OtherComp :type Primitive%20Component%20Object%20Reference) (OtherBodyIndex :type Integer))
  (Widget|SetVisibility (Variables|/Game/Widget/UserWidget.UserWidget_C|GetDoor (Variables|Default|GetWidget)) "Hidden")
  (Input|DisableInput (Game|GetPlayerController 0)))

(event Custom|Close%20Door
  (bind _newtrack_0 (Timeline|Door%20Anim Reverse)
    (:Update
      (Transformation|SetRelativeLocation (Variables|Default|GetStaticMesh) (Math|Vector|Lerp(Vector) "0, 0, 0" "-85.000000,0.000000,0.000000" _newtrack_0) false false))))

(event Custom|Open%20Door
  (bind _newtrack_0 (Timeline|Door%20Anim PlayFromStart)
    (:Update
      (Transformation|SetRelativeLocation (Variables|Default|GetStaticMesh) (Math|Vector|Lerp(Vector) "0, 0, 0" "-85.000000,0.000000,0.000000" _newtrack_0) false false))))

(event Input|EnhancedActionEvents|EnhancedInputActionIA_Interaction
  (params (ActionValue :type Boolean) (ElapsedSeconds :type Float%20%28double-precision%29) (TriggeredSeconds :type Float%20%28double-precision%29) (InputAction :type Input%20Action%20Object%20Reference :default "/Game/ThirdPerson/Input/Actions/IA_Interaction.IA_Interaction"))
  (:Started
    (Utilities|FlowControl|FlipFlop
      (:A
        (CallFunction|OpenDoor)
        (Variables|Default|SetIsOpen? true)
        (Utilities|FlowControl|Delay 0.5))
      (:B
        (CallFunction|CloseDoor)
        (Variables|Default|SetIsOpen? false)
        (Utilities|FlowControl|Delay 0.5)))))

(event EventBeginPlay
  (bind _returnvalue (UserInterface|CreateWidget "/Game/Widget/UserWidget.UserWidget_C"))
  (bind _output_get (Variables|Default|SetWidget _returnvalue))
  (UserInterface|Viewport|AddtoViewport _output_get 0))

(event Collision|EventActorBeginOverlap
  (params (OtherActor :type Actor%20Object%20Reference)))

(event EventTick
  (params (DeltaSeconds :type Float%20%28single-precision%29))
  (if (Variables|Default|GetIsOpen?)
    (Widget|SetVisibility (Variables|/Game/Widget/UserWidget.UserWidget_C|GetDoor (Variables|Default|GetWidget)) "Hidden")))

(event EventEndPlay
  (params (EndPlayReason :type EEndPlayReason%20Enum :default "Destroyed"))
  (Widget|RemovefromParent (Variables|Default|GetWidget)))

(fn ConstructionScript)