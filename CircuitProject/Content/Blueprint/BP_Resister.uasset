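; BP_Resister is a placeable Blueprint, apparently a resistor, with two child-actor end points on a cell-based field.
; The construction script offsets LeftActor and RightActor one cell length (FieldLength / CellCount) to either side along Y and caches their child actors as LeftPoint and RightPoint.
; DetachCHildActor forwards DetachMessage to both child actors, while BeginPlay only calls the parent.
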(event EventBeginPlay
  (|CallParentFunction))

(event Collision|EventActorBeginOverlap
  (params (OtherActor :type Actor%20Object%20Reference))
  (|CallParentFunction OtherActor) ; 지금 이 노드는 비활성 상태입니다. \n핀을 끌어서 다른 노드를 연결하면 활성화됩니다.
)

(event EventTick
  (params (DeltaSeconds :type Float%20%28single-precision%29))
  (|CallParentFunction DeltaSeconds) ; 지금 이 노드는 비활성 상태입니다. \n핀을 끌어서 다른 노드를 연결하면 활성화됩니다.
)

(event EventDetachCHildActor
  (Class|Attach|Detach(Message) (Variables|/Script/Engine.ChildActorComponent|GetChildActor (Variables|Default|GetLeftActor)))
  (Class|Attach|Detach(Message) (Variables|/Script/Engine.ChildActorComponent|GetChildActor (Variables|Default|GetRightActor))))

(fn ConstructionScript
  (bind _fieldlength (Variables|Default|GetFieldLength))
  (bind _cellcount (Variables|Default|GetcellCount))
  (bind _returnvalue (/ _fieldlength _cellcount))
  (|CallParentFunction)
  (Transformation|SetRelativeLocation (Variables|Default|GetLeftActor) (Math|Vector|MakeVector 0.0 _returnvalue 0.0) false false)
  (Transformation|SetRelativeLocation (Variables|Default|GetRightActor) (Math|Vector|MakeVector 0.0 (* _returnvalue -1.0) 0.0) false false)
  (Variables|Default|SetLeftPoint (Variables|/Script/Engine.ChildActorComponent|GetChildActor (Variables|Default|GetLeftActor)))
  (Variables|Default|SetRightPoint (Variables|/Script/Engine.ChildActorComponent|GetChildActor (Variables|Default|GetRightActor))))