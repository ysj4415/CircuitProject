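; Selectable, movable actor, apparently mouse-driven, that can attach to and detach from other actors and is sized to one field cell.
; Select and CancleSelect toggle custom-depth highlighting, while Move eases it toward a given location when allowed.
; AttachComponent snaps it to the actor returned by the target's check, registers with that parent and disables sphere collision.
; Detach releases the newest child, which restores its collision and nudges itself aside.
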(event EventBeginPlay)

(event Collision|EventActorBeginOverlap
  (params (OtherActor :type Actor%20Object%20Reference)))

(event EventTick
  (params (DeltaSeconds :type Float%20%28single-precision%29)))

(event EventCancleSelect
  (Rendering|SetRenderCustomDepth (Variables|Default|GetStaticMesh) false))

(event EventMove
  (params (Location :type Vector :default "0, 0, 0"))
  (if (Variables|Default|Getcanmove)
    (Transformation|SetActorLocation (Math|Interpolation|VInterpTo (Transformation|GetActorLocation) Location (Utilities|Time|GetWorldDeltaSeconds) 8.0) false false)))

(event EventMessagetoAttach
  (params (NewParam :type Actor%20Object%20Reference))
  (Utilities|Array|Add (Variables|Default|GetAttachactor%20to%20me) NewParam))

(fn ConstructionScript
  (bind _fieldlength (Variables|Default|GetFieldLength))
  (bind _cellcount (Variables|Default|GetcellCount))
  (bind _returnvalue (Utilities|Operators|Divide _fieldlength _cellcount 1e+01))
  (Transformation|SetWorldScale3D (Variables|Default|GetStaticMesh) (Math|Vector|MakeVector _returnvalue _returnvalue _returnvalue)))

(fn AttachComponent
  (params (AttachActor :type Actor%20Object%20Reference))
  (if (Variables|Default|Getcanattach)
    (bind _targetactor (Class|Attach|CheckAttach(Message) AttachActor))
    (bind _returnvalue (Transformation|AttachActorToActor _targetactor "None" "SnapToTarget" "SnapToTarget" "KeepWorld" true))
    (if _returnvalue
      (bind _output_get (Variables|Default|SetAttachActor _targetactor))
      (Class|Attach|MessagetoAttach(Message) _output_get self)
      (Collision|SetCollisionEnabled (Variables|Default|GetSphere) "NoCollision")
      (return true))))

(fn CheckAttach
  (if (Variables|Default|Getcanattached)
    (return self)))

(fn Detach
  (bind _attachactor_to_me (Variables|Default|GetAttachactor%20to%20me))
  (bind _attachactor_to_me_2 (Variables|Default|GetAttachactor%20to%20me))
  (if (Utilities|Array|IsNotEmpty _attachactor_to_me)
    (Class|Attach|DetachfromMe(Message) (Utilities|Array|Get(acopy) _attachactor_to_me (Utilities|Array|LastIndex _attachactor_to_me)))
    (Utilities|Array|RemoveIndex _attachactor_to_me_2 (Utilities|Array|LastIndex _attachactor_to_me_2))
    (return)))

(fn DetachfromMe
  (Transformation|DetachFromActor "KeepWorld" "KeepWorld" "KeepWorld")
  (Collision|SetCollisionEnabled (Variables|Default|GetSphere) "QueryOnly")
  (Variables|Default|SetAttachActor 0)
  (Transformation|AddActorLocalOffset "20.000000,0.000000,0.000000" false false))

(fn Select
  (Rendering|SetRenderCustomDepth (Variables|Default|GetStaticMesh) true)
  (return self))