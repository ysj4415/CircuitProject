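; Mouse controller for selecting, dragging, rotating and attaching objects under a visible cursor using Enhanced Input.
; A press traces under the cursor to change the selection, messaging the actor and notifying the widget.
; Holding drags it along WorldStatic hits, with a gate blocking movement during the press that changed selection.
; Release attempts attachment to the actor under the cursor, deselecting on success; rotate input turns yaw and X detaches.
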(event Input|EnhancedActionEvents|EnhancedInputActionIA_SelectObject
  (params (ActionValue :type Boolean) (ElapsedSeconds :type Float%20%28double-precision%29) (TriggeredSeconds :type Float%20%28double-precision%29) (InputAction :type Input%20Action%20Object%20Reference :default "/Game/Blueprint/Input/IA_SelectObject.IA_SelectObject"))
  (bind _hitresult (Game|Player|GetHitResultUnderCursorbyChannel "TraceTypeQuery3" true))
  (bind _hitresult_2 (Game|Player|GetHitResultUnderCursorbyChannel "TraceTypeQuery4" true))
  (bind (_bblockinghit _binitialoverlap _time _distance _location _impactpoint _normal _impactnormal _physmat _hitactor) (Collision|BreakHitResult _hitresult_2))
  (bind _hitactor_2 (Collision|BreakHitResult _hitresult))
  (:Triggered
    (Utilities|FlowControl|Gate true :!label _label
      (:Exit
        (Utilities|IsValid (Variables|Default|GetSelectObject)
          (:Is%20Valid
            (Class|BPSelectModeInterface|Move(Message) (Variables|Default|GetSelectObject) (.Location (Collision|BreakHitResult (.HitResult (Class|PlayerController|GetHitResultUnderCursorforObjects (Utilities|Array|MakeArray "ObjectTypeQuery1") true))))))))))
  (:Started
    (if _bblockinghit
      (bind _targetactor (Class|BPSelectModeInterface|Select(Message) _hitactor))
      (if (not (== _targetactor (Variables|Default|GetSelectObject)))
        (Class|BPSelectModeInterface|CancleSelect(Message) (Variables|Default|GetSelectObject) :!label _label_2)
        (Variables|Default|SetSelectObject _targetactor)
        (Default|SelectObjectEvent (Variables|Default|GetWidget))
        (goto _label Close))
      (else
        (Utilities|FlowControl|Sequence
          (:then_0
            (goto _label_2))))))
  (:Completed
    (if (!= (Variables|Default|GetSelectObject) _hitactor_2)
      (bind _ok (Class|Attach|AttachComponent(Message) (Variables|Default|GetSelectObject) _hitactor_2))
      (if _ok
        (Class|BPSelectModeInterface|CancleSelect(Message) (Variables|Default|GetSelectObject))
        (Variables|Default|SetSelectObject 0)
        (goto _label Open)
        (else
          (goto _label Open)))
      (else
        (goto _label Open)))))

(event Input|EnhancedActionEvents|EnhancedInputActionIA_RotateObject
  (params (ActionValue :type Float%20%28double-precision%29) (ElapsedSeconds :type Float%20%28double-precision%29) (TriggeredSeconds :type Float%20%28double-precision%29) (InputAction :type Input%20Action%20Object%20Reference :default "/Game/Blueprint/Input/IA_RotateObject.IA_RotateObject"))
  (bind _selectobject (Variables|Default|GetSelectObject))
  (:Triggered
    (Transformation|SetActorRotation _selectobject (Math|Rotator|MakeRotator 0.0 0.0 (+ (.yaw (Transformation|GetActorRotation _selectobject)) (* ActionValue (Variables|Default|GetRotateSpeed)))))))

(event EventBeginPlay
  (Input|AddMappingContext (PlayerController|LocalPlayerSubsystems|GetEnhancedInputLocalPlayerSubsystem) "/Game/Blueprint/Input/IMC_SelectInput.IMC_SelectInput" 0 "(bIgnoreAllPressedKeysUntilRelease=True,bForceImmediately=False)")
  (Variables|Default|SetbShowMouseCursor true))

(event EventTick
  (params (DeltaSeconds :type Float%20%28single-precision%29)))

(event Input|KeyboardEvents|X
  (params (Key :type Key%20Structure :default "None"))
  (bind _selectobject (Variables|Default|GetSelectObject))
  (:Pressed
    (Utilities|IsValid _selectobject
      (:Is%20Valid
        (Class|Attach|Detach(Message) _selectobject)))))

(fn ConstructionScript)