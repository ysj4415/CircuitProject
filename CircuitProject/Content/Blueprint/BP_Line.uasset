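; BP_Line is an actor that draws a cable between two child actors, StartPoint and EndPoint.
; The construction script caches both child actors as LeftPoint and RightPoint.
; BeginPlay attaches the cable's end to the EndPoint actor, and Tick moves the cable's origin to the StartPoint actor's location every frame.
; A destroy_1 event destroys the whole line actor.
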(event Custom|destroy_1
  (Actor|DestroyActor))

(event EventBeginPlay
  (Class|CableComponent|SetAttachEndto (Variables|Default|GetCable) (Variables|/Script/Engine.ChildActorComponent|GetChildActor (Variables|Default|GetEndPoint)) "None" "None"))

(event Collision|EventActorBeginOverlap
  (params (OtherActor :type Actor%20Object%20Reference)))

(event EventTick
  (params (DeltaSeconds :type Float%20%28single-precision%29))
  (CallFunction|SetCableLocation))

(fn ConstructionScript
  (Variables|Default|SetLeftPoint (Variables|/Script/Engine.ChildActorComponent|GetChildActor (Variables|Default|GetStartPoint)))
  (Variables|Default|SetRightPoint (Variables|/Script/Engine.ChildActorComponent|GetChildActor (Variables|Default|GetEndPoint))))

(fn SetCableLocation
  (Transformation|SetWorldLocation (Variables|Default|GetCable) (Transformation|GetActorLocation (Variables|/Script/Engine.ChildActorComponent|GetChildActor (Variables|Default|GetStartPoint))) false false))